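; BP_Movable is a cube actor that fan wind pushes and that, while zoom is on, grows or shrinks as the player approaches or retreats.
; BeginPlay finds maximum size by stepping scale up until a box trace hits, then saves the transform for Reset.
; Resizing sends UnlockedMessage to traced actors.
; Wind box-traces ahead, destroying hit enemies or, if clear, moving the cube, with smaller scale extending effective range.
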(event Custom|Reset
  (Transformation|SetActorTransform (Variables|Default|GetInitial%20Data)))

(event EventBeginPlay
  (bind _returnvalue (Transformation|GetActorLocation))
  (Variables|Default|Set初始大小 (.x (Transformation|GetActorScale3D)))
  (Utilities|FlowControl|ForLoopwithBreak 0 19 :!label _label
    (:LoopBody
      (Transformation|SetActorScale3D (+ (Transformation|GetActorScale3D) 0.1))
      (bind _returnvalue_2 (Class|KismetSystemLibrary|BoxTraceMulti _returnvalue _returnvalue (.BoxExtent (Collision|GetComponentBounds (Variables|Default|GetCube))) "0, 0, 0" "TraceTypeQuery1" false 0 "None" true))
      (if _returnvalue_2
        (goto _label Break)))
    (:Completed
      (Variables|Default|Set最大大小 (.x (Transformation|GetActorScale3D)))
      (Transformation|SetActorScale3D (Math|Conversions|ToVector(Float) (Variables|Default|Get当前尺寸)))
      (Variables|Default|SetInitial%20Data (Transformation|GetActorTransform)))))

(event Collision|EventActorBeginOverlap
  (params (OtherActor :type Actor%20Object%20Reference)))

(event EventTick
  (params (DeltaSeconds :type Float%20%28single-precision%29))
  (bind _returnvalue (Transformation|GetActorLocation))
  (if (Variables|Default|Get开始缩放)
    (if (Math|Float|InRange(Float) (+ (.X (Math|Vector|BreakVector (Transformation|GetActorScale3D))) (* (- (Variables|Default|Get初始距离) (Math|Vector|VectorLength (- (Transformation|GetActorLocation) (Transformation|GetActorLocation (Game|GetPlayerCharacter 0))))) 0.0005)) (Variables|Default|Get最小尺寸) (Variables|Default|Get最大大小))
      (Transformation|SetActorScale3D (Math|Conversions|ToVector(Float) (+ (.X (Math|Vector|BreakVector (Transformation|GetActorScale3D))) (* (- (Variables|Default|Get初始距离) (Math|Vector|VectorLength (- (Transformation|GetActorLocation) (Transformation|GetActorLocation (Game|GetPlayerCharacter 0))))) 0.0005))))
      (Variables|Default|Set初始距离 (Math|Vector|VectorLength (- (Transformation|GetActorLocation) (Transformation|GetActorLocation (Game|GetPlayerCharacter 0)))))
      (bind _outhit (Collision|BoxTraceByChannel _returnvalue _returnvalue (.BoxExtent (Collision|GetComponentBounds (Variables|Default|GetCube))) "0, 0, 0" "TraceTypeQuery1" false 0 "None"))
      (Class|IBPPuzzleInterface|Unlocked(Message) (.HitActor (Collision|BreakHitResult _outhit))))))

(fn ConstructionScript
  (if (Variables|Default|Get预览最小尺寸)
    (Transformation|SetActorScale3D (Math|Conversions|ToVector(Float) (Variables|Default|Get最小尺寸)))
    (else
      (Transformation|SetActorScale3D (Math|Conversions|ToVector(Float) (Variables|Default|Get当前尺寸))))))

(fn ReceiveWindForceFields
  (params (Fan :type BP%20Fan%20Object%20Reference))
  (bind _cube (Variables|Default|GetCube))
  (bind (_origin _boxextent _sphereradius) (Collision|GetComponentBounds _cube))
  (bind (_outhits _returnvalue) (Class|KismetSystemLibrary|BoxTraceMulti (Transformation|GetActorLocation) (+ _origin (* (Transformation|GetActorForwardVector Fan) (* (Variables|Default|Get%20StepSize_M) _sphereradius))) _boxextent "0, 0, 0" "TraceTypeQuery1" false 0 "ForOneFrame" true))
  (if _returnvalue
    (for _array_element _outhits
      (bind _asbp_enemy (Utilities|Casting|CastToBP_Enemy (.HitActor (Collision|BreakHitResult _array_element))))
      (Actor|DestroyActor _asbp_enemy))
    (elif (> (/ (Variables|Default|Get最小尺寸) (.X (Math|Vector|BreakVector (Transformation|GetActorScale3D)))) (/ (Math|Vector|VectorLength (- (Transformation|GetActorLocation Fan) (Transformation|GetActorLocation))) (Variables|/Game/Game/Blueprint/Fan/BP_Fan.BP_Fan_C|GetWind%20Range%20Distance Fan)))
      (Transformation|SetActorLocation (+ (Transformation|GetActorLocation) (* (* (Math|Vector|GetForwardVector (Variables|/Game/Game/Blueprint/Fan/BP_Fan.BP_Fan_C|GetArrow Fan)) (Variables|Default|GetMoveSpeed)) (LocalVariables|GetTimerInterval))) false false))))

(fn TurnonZoom
  (params (开始缩放 :type Boolean))
  (Variables|Default|Set开始缩放 开始缩放)
  (Variables|Default|Set初始距离 (Math|Vector|VectorLength (- (Transformation|GetActorLocation) (Transformation|GetActorLocation (Game|GetPlayerCharacter 0))))))